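; BP_Clock is an in-game clock that advances an accelerated time of day and counts elapsed days.
; Each Tick, ClockTrue accumulates delta time scaled by DayLenght and a fixed multiplier, then converts it to a Timespan.
; It pushes an unpadded hours:minutes Name to BP_FirstPersonCharacter, updating DayCount only when that cast succeeds.
; Day and OutputTime expose the day count and current hour.
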(event `self.ReceiveTick`
  (params (DeltaSeconds :type "Float (single-precision)"))
  (`self.ClockTrue` (* DeltaSeconds (`self.Day Lenght`)))
  (set `self.CurrentTime` (`self.Time`)))

(fn `ClockTrue`
  (params (Delta :type "Float (double-precision)"))
  (bind _output_get (set `self.Tick` (+ (* Delta 240.0) (`self.Tick`))))
  (bind _output_get_2 (set `self.Time` (`KismetMathLibrary.MakeTimespan` 0 0 0 (`KismetMathLibrary.FTrunc` _output_get))))
  (bind _asbp_first_person_character (cast `/Game/AIENEMYCONTENTANDMAP/AI_And_FirstPerson/Blueprints/BP_FirstPersonCharacter` (`GameplayStatics.GetPlayerCharacter` 0)))
  (bind (_days _hours _minutes) (`KismetMathLibrary.BreakTimespan` _output_get_2))
  (set `/Game/AIENEMYCONTENTANDMAP/AI_And_FirstPerson/Blueprints/BP_FirstPersonCharacter.Time` (`KismetStringLibrary.Conv_StringToName` (`KismetStringLibrary.Concat_StrStr` (`KismetStringLibrary.Conv_IntToString` _hours) ":" (`KismetStringLibrary.Conv_IntToString` _minutes))) _asbp_first_person_character)
  (set `self.DayCount` _days))

(fn `Day`
  (returns (DayCount :type Integer))
  (return (`self.DayCount`)))

(fn `OutputTime`
  (returns (CurrentTime :type Integer))
  (return (`.Hours` (`KismetMathLibrary.BreakTimespan` (`self.CurrentTime`)))))

(fn `UserConstructionScript`)