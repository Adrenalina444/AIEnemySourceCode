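; BP_TimePrint is an actor that prints a time value on screen when the first-person character overlaps it.
; On begin overlap, it casts to BP_FirstPersonCharacter, queries its TimeActor reference through OutputTimeMessage, and prints the result only if it is at least TimeToUse.
; Its own Day and OutputTime functions are stubs that return zero, and the construction script is empty.
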(event `self.ReceiveActorBeginOverlap`
  (params (OtherActor :type "Actor Object Reference"))
  (cast `/Game/AIENEMYCONTENTANDMAP/AI_And_FirstPerson/Blueprints/BP_FirstPersonCharacter` OtherActor)
  (bind _currenttime (message `/Game/BPI_Clock.OutputTime` (`self.TimeActor`)))
  (if (>= _currenttime (`self.TimeToUse`))
    (`KismetSystemLibrary.PrintString` (`KismetStringLibrary.Conv_IntToString` _currenttime))))

(fn `Day`
  (returns (DayCount :type Integer))
  (return 0))

(fn `OutputTime`
  (returns (CurrentTime :type Integer))
  (return 0))

(fn `UserConstructionScript`)