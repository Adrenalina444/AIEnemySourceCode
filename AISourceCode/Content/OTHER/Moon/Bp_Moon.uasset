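; Moon actor Blueprint that fades a moon, its glow and its directional light between day and night.
; NightTransition plays the DayToNight timeline, driving the moon material's Opacity, the glow's Density and the light's intensity.
; DayTransition reverses the same timeline.
; The construction script aims the actor at an Origin point and applies a uniform Scale.
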(event `NightTransition`
  (bind (_direction _moon _glow _directionallight) (`Timeline|DayToNight` :!label _label)
    (:`Update`
      (`MeshComponent.SetScalarParameterValueOnMaterials` (`self.Moon`) "Opacity" _moon)
      (`MeshComponent.SetScalarParameterValueOnMaterials` (`self.Glow`) "Density" _glow)
      (`LightComponent.SetIntensity` (`self.DirectionalLight`) _directionallight))))

(event `Day Transition`
  (goto _label :!via `Reverse`))

(fn `UserConstructionScript`
  (bind _scale (`self.Scale`))
  (`self.K2_SetActorRotation` (`KismetMathLibrary.Conv_VectorToRotator` (`KismetMathLibrary.Normal` (- (`self.Origin`) (`self.K2_GetActorLocation`)))))
  (`self.SetActorScale3D` (`KismetMathLibrary.MakeVector` _scale _scale _scale)))